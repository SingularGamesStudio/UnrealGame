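; Character component that provides animation data: look direction, attacking state and flipped state.
; Look direction points at Target when valid, otherwise along the owner's forward vector.
; With ForceLookRotation on, Tick yaws the mesh from its initial rotation by the negated, ±90-clamped look-to-velocity angle, orienting it for the animation blendspace, which players don't need.
; It also draws a debug arrow of the look direction on authority.
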(event EventBeginPlay
  (bind _ascharacter (Utilities|Casting|CastToCharacter (Components|GetOwner)))
  (bind _output_get (Variables|Default|SetCharacter _ascharacter))
  (Variables|Default|SetInitialRotation (.Yaw (Math|Rotator|BreakRotator (Variables|/Script/Engine.SceneComponent|GetRelativeRotation (Variables|/Script/Engine.Character|GetMesh _output_get))))))

(event EventTick
  (params (DeltaSeconds :type Float%20%28single-precision%29))
  (bind _returnvalue (Components|GetOwner))
  (bind _character (Variables|Default|GetCharacter))
  (bind _returnvalue_2 (Transformation|GetActorLocation _returnvalue))
  (bind _charactermovement (Variables|/Script/Engine.Character|GetCharacterMovement _character))
  (bind _velocity (Variables|/Script/Engine.MovementComponent|GetVelocity _charactermovement))
  (bind (_x _y) (Math|Vector|BreakVector _velocity))
  (bind _returnvalue_3 (Math|Vector|MakeVector _x _y 0.0))
  (bind _returnvalue_4 (Math|Vector|Normalize _returnvalue_3))
  (if (Variables|Default|GetForceLookRotation)
    ;[0.15 0.15 0.15 0.5] Mesh must be oriented towards look direction for animation blendspace to work correctly (already true for player)
    (bind _forward (CallFunction|GetLookDirection))
    (Transformation|SetRelativeRotation (Variables|/Script/Engine.Character|GetMesh (Variables|Default|GetCharacter)) (Math|Rotator|MakeRotator 0.0 0.0 (+ (* (Math|Float|Clamp(Float) (Class|KismetMathLibrary|DegAtan2 (Class|KismetMathLibrary|CrossProduct2D (Math|Conversions|ToVector2D(Vector) (Math|Vector|Normalize (Math|Vector|MakeVector (.X (Math|Vector|BreakVector _forward)) (.Y (Math|Vector|BreakVector _forward)) 0.0))) (Math|Conversions|ToVector2D(Vector) _returnvalue_4)) (Math|Vector|DotProduct (Math|Vector|Normalize (Math|Vector|MakeVector (.X (Math|Vector|BreakVector _forward)) (.Y (Math|Vector|BreakVector _forward)) 0.0)) _returnvalue_4)) -9e+01 9e+01) -1.0) (Variables|Default|GetInitialRotation))) false false)
    (Networking|SwitchHasAuthority
      (:Authority
        (Rendering|Debug|DrawDebugArrow :LineStart _returnvalue_2 :LineEnd (+ _forward _returnvalue_2) :ArrowSize 1e+02)))))

(fn IsFlipped
  (return (Variables|Default|GetFlipped)))

(fn GetLookDirection
  (bind _returnvalue (Components|GetOwner))
  (bind _target (Variables|Default|GetTarget))
  (Utilities|IsValid _target
    (:Is%20Valid
      (return (- (Transformation|GetActorLocation _target) (Transformation|GetActorLocation _returnvalue))))
    (:Is%20Not%20Valid
      (return (Transformation|GetActorForwardVector _returnvalue)))))

(fn IsAttacking
  (return (Variables|Default|GetAttacking)))