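; AI controller for BP_AttackerCharacter enemies that picks perceived hostiles as focus and chases them.
; A looping timer randomly switches or reacquires targets, and perception updates retarget when focus is empty.
; Each tick, Chase pathfinds to the focus, or moves directly while falling, and charges a jump when slowed until it can reach the target's height.
; An attack event handles animation timing and cooldown, but its range-check trigger is disconnected.
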(event Custom|ChangeTarget
  (CallFunction|FChangeTarget))

(event Custom|PerceptionUpdated
  (params (UpdatedActors :type Array%20of%20Actor%20Object%20References))
  ;[0.15 0.15 0.15 0.5] if no focus, receiving stimuli instantly looks for one
  (Utilities|IsValid (Class|AIController|GetFocusActor)
    (:Is%20Not%20Valid
      (CallFunction|FChangeTarget))))

(event Custom|Attack
  (bind _possessed (Variables|Default|GetPossessed))
  (if (not (Variables|Default|GetAttackOnCooldown))
    (Variables|Default|SetAttackOnCooldown true)
    (Variables|/Game/Blueprints/BP_AttackerCharacter.BP_AttackerCharacter_C|SetAttacking _possessed true)
    (Utilities|FlowControl|Delay (Animation|GetPlayLength (Variables|Default|GetAttackAnim)))
    (Variables|/Game/Blueprints/BP_AttackerCharacter.BP_AttackerCharacter_C|SetAttacking _possessed false)
    (Utilities|FlowControl|Delay (Variables|Default|GetAttackCooldown))
    (Variables|Default|SetAttackOnCooldown false)))

(event EventBeginPlay)

(event EventTick
  (params (DeltaSeconds :type Float%20%28single-precision%29))
  (CallFunction|FTick DeltaSeconds))

(event EventPossess
  (params (PossessedPawn :type Pawn%20Object%20Reference))
  (bind _asbp_attacker_character (Utilities|Casting|CastToBP_AttackerCharacter PossessedPawn))
  (bind _output_get (Variables|Default|SetPossessed _asbp_attacker_character))
  (bind _output_get_2 (Variables|Default|SetMovement (Variables|/Script/Engine.Character|GetCharacterMovement _output_get)))
  (Variables|Default|SetBaseJumpVel (Variables|/Script/Engine.CharacterMovementComponent|GetJumpZVelocity _output_get_2))
  (Variables|Default|SetAttackAnim (Variables|/Game/Blueprints/BP_AttackerCharacter.BP_AttackerCharacter_C|GetAttackAnim _output_get))
  (CallFunction|ChangeTarget)
  (Utilities|Time|SetTimerbyEvent (delegate Custom|ChangeTarget) 1e+01 true)
  (EventDispatchers|BindEventtoOnPerceptionUpdated (Class|AIController|GetAIPerceptionComponent) (delegate Custom|PerceptionUpdated)))

(fn ConstructionScript)

(fn FChangeTarget
  (bind _returnvalue (Class|AIController|GetFocusActor))
  (bind _returnvalue_2 (Class|AIController|GetAIPerceptionComponent))
  (bind _outactors (Class|AIPerceptionComponent|GetPerceivedHostileActors _returnvalue_2))
  (bind _returnvalue_3 (Utilities|Array|FindItem _outactors _returnvalue))
  (bind _returnvalue_4 (Utilities|Array|Length _outactors))
  (bind _returnvalue_5 (- _returnvalue_4 1))
  (bind _returnvalue_6 (!= _returnvalue_3 -1))
  (bind _returnvalue_7 (Math|Random|RandomInteger _returnvalue_5))
  (Utilities|IsValid _returnvalue
    (:Is%20Valid
      (if _returnvalue_6
        (Math|Float|CompareFloat (Math|Random|RandomFloat) (Variables|Default|GetTargetSwitchChance)
          (:<
            _))))
    (:Is%20Not%20Valid
      _))
  (if (> (Utilities|Array|Length _outactors) _returnvalue_6)
    ;[0.15 0.15 0.15 0.5] random visible actor, except the current focus
    (AI|SetFocus (Utilities|Array|Get(acopy) _outactors (+ _returnvalue_7 (and (>= _returnvalue_7 _returnvalue_3) (!= _returnvalue_3 -1)))))
    (Variables|/Game/Blueprints/BP_AttackerCharacter.BP_AttackerCharacter_C|SetTarget (Variables|Default|GetPossessed) (Class|AIController|GetFocusActor))
    (else
      (AI|SetFocus)
      (Variables|/Game/Blueprints/BP_AttackerCharacter.BP_AttackerCharacter_C|SetTarget (Variables|Default|GetPossessed) 0))))

(fn FTick
  (params (deltaTime :type Float%20%28double-precision%29))
  (Utilities|IsValid (Class|AIController|GetFocusActor)
    (:Is%20Valid
      (switch Utilities|FlowControl|Switch|SwitchonEnemyCombatBehavior (Variables|Default|GetCombatBehavior)
        (:NewEnumerator0
          (CallFunction|Chase deltaTime))))
    (:Is%20Not%20Valid
      (switch Utilities|FlowControl|Switch|SwitchonEnemyIdleBehavior (Variables|Default|GetIdleBehavior)))))

(fn Chase
  (params (deltaTime :type Float%20%28double-precision%29))
  (bind _returnvalue (Class|AIController|GetFocusActor))
  (bind _possessed (Variables|Default|GetPossessed))
  (Utilities|FlowControl|Sequence
    (:then_0
      (bind _returnvalue_2 (AI|Components|NavMovement|IsFalling (Variables|Default|GetMovement)))
      (if _returnvalue_2
        (AI|Navigation|MovetoActor _returnvalue -1.0 true false true 0)
        (else
          (bind _returnvalue_3 (AI|Navigation|MovetoActor _returnvalue -1.0 true true true 0))
          ;[0.15 0.15 0.15 0.5] On unreached partial path, try to jump (charged)
          (switch Utilities|FlowControl|Switch|SwitchonEPathFollowingRequestResult _returnvalue_3
            (:Failed
              _)
            (:RequestSuccessful
              _))
          (Math|Float|CompareFloat (Math|Vector|VectorLength (Variables|/Script/Engine.MovementComponent|GetVelocity (Variables|Default|GetMovement))) (Variables|Default|GetVelocityThreshold)
            (:>
              (Variables|Default|SetJumpCharge 0.0 :!label _label))
            (:==
              (goto _label))
            (:<
              (bind _output_get (Variables|Default|SetJumpCharge (+ (Variables|Default|GetJumpCharge) deltaTime)))
              (Math|Float|CompareFloat _output_get (Variables|Default|GetMinJumpDelay)
                (:>
                  (Math|Float|CompareFloat (Utilities|Operators|Divide (Math|Float|Square (* _output_get (Variables|Default|GetBaseJumpVel))) 2.0 (Math|Float|Absolute(Float) (Components|Movement|GetGravityZ (Variables|Default|GetMovement)))) (- (.Z (Math|Vector|BreakVector (Transformation|GetActorLocation (Class|AIController|GetFocusActor)))) (- (.Z (Math|Vector|BreakVector (Transformation|GetActorLocation _possessed))) (Variables|/Script/Engine.CapsuleComponent|GetCapsuleHalfHeight (Variables|/Script/Engine.Character|GetCapsuleComponent _possessed))))
                    (:>
                      (Variables|/Script/Engine.CharacterMovementComponent|SetJumpZVelocity (Variables|Default|GetMovement) (* _output_get (Variables|Default|GetBaseJumpVel)))
                      (Character|Jump (Variables|Default|GetPossessed))
                      (Variables|Default|SetJumpCharge 0.0))))))))))))