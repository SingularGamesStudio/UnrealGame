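; Golem enemy Blueprint that deals melee damage during attacks and destroys itself on death after running the parent logic.
; While Attacking, the server polls Hitbox overlaps every Tick and applies PowerfulDamage to each newly found actor.
; AddUnique's returned index, checked with IsValidIndex, limits hits to one per actor until the Damaged list clears when not attacking.
; The construction script assigns a PumpkinCreature unarmed attack animation.
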(event EventBeginPlay
  (|CallParentFunction))

(event Collision|EventActorBeginOverlap
  (params (OtherActor :type Actor%20Object%20Reference)))

(event EventTick
  (params (DeltaSeconds :type Float%20%28single-precision%29))
  (bind _damaged (Variables|Default|GetDamaged))
  (|CallParentFunction DeltaSeconds)
  (Networking|SwitchHasAuthority
    (:Authority
      (if (Variables|Default|GetAttacking)
        (for _array_element (Collision|GetOverlappingActors (Variables|Default|GetHitbox) 0 :!class /Script/Engine.PrimitiveComponent)
          (bind _returnvalue (Utilities|Array|AddUnique _damaged _array_element))
          (if (Utilities|Array|IsValidIndex _damaged _returnvalue)
            (Game|Damage|ApplyDamage _array_element (Variables|Default|GetDamage) (Pawn|GetController) self "/Game/Blueprints/PowerfulDamage.PowerfulDamage_C")))
        (else
          (Utilities|Array|Clear (Variables|Default|GetDamaged)))))))

(fn ConstructionScript
  (Variables|Default|SetAttackAnim "/Game/StylizedHalloweenPack/Animations/PumpkinCreature/A_PumpkinCreature_Combat_Unarmed_Attack01.A_PumpkinCreature_Combat_Unarmed_Attack01"))

(fn OnDeath
  (|CallParentFunction)
  (Actor|DestroyActor))