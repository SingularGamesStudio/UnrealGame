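; BP_AttackerCharacter is a character that keeps its mesh facing its look direction while moving, as its animation blendspace requires.
; Look direction points at Target when valid, otherwise along actor forward.
; Each tick offsets the mesh's initial yaw by the negated, clamped signed 2D angle between look direction and velocity.
; Authority also draws a debug look arrow, and simple getters expose the Attacking and Flipped states.
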(event EventBeginPlay
  (Variables|Default|SetInitialRotation (.Yaw (Math|Rotator|BreakRotator (Variables|/Script/Engine.SceneComponent|GetRelativeRotation (Variables|Character|GetMesh))))))

(event Collision|EventActorBeginOverlap
  (params (OtherActor :type Actor%20Object%20Reference)))

(event EventTick
  (params (DeltaSeconds :type Float%20%28single-precision%29))
  (bind _returnvalue (Transformation|GetActorLocation))
  (bind _charactermovement (Variables|Character|GetCharacterMovement))
  (bind _velocity (Variables|/Script/Engine.MovementComponent|GetVelocity _charactermovement))
  (bind (_x _y) (Math|Vector|BreakVector _velocity))
  (bind _returnvalue_2 (Math|Vector|MakeVector _x _y 0.0))
  (bind _returnvalue_3 (Math|Vector|Normalize _returnvalue_2))
  ;[0.15 0.15 0.15 0.5] Mesh must be oriented towards look direction for animation blendspace to work correctly (already true for player)
  (bind _forward (CallFunction|GetLookDirection))
  (Transformation|SetRelativeRotation (Variables|Character|GetMesh) (Math|Rotator|MakeRotator 0.0 0.0 (+ (* (Math|Float|Clamp(Float) (Class|KismetMathLibrary|DegAtan2 (Class|KismetMathLibrary|CrossProduct2D (Math|Conversions|ToVector2D(Vector) (Math|Vector|Normalize (Math|Vector|MakeVector (.X (Math|Vector|BreakVector _forward)) (.Y (Math|Vector|BreakVector _forward)) 0.0))) (Math|Conversions|ToVector2D(Vector) _returnvalue_3)) (Math|Vector|DotProduct (Math|Vector|Normalize (Math|Vector|MakeVector (.X (Math|Vector|BreakVector _forward)) (.Y (Math|Vector|BreakVector _forward)) 0.0)) _returnvalue_3)) -9e+01 9e+01) -1.0) (Variables|Default|GetInitialRotation))) false false)
  (Networking|SwitchHasAuthority
    (:Authority
      (Rendering|Debug|DrawDebugArrow :LineStart _returnvalue :LineEnd (+ _forward _returnvalue) :ArrowSize 1e+02))))

(fn ConstructionScript)

(fn GetLookDirection
  (bind _target (Variables|Default|GetTarget))
  (Utilities|IsValid _target
    (:Is%20Valid
      (return (- (Transformation|GetActorLocation _target) (Transformation|GetActorLocation))))
    (:Is%20Not%20Valid
      (return (Transformation|GetActorForwardVector)))))

(fn IsAttacking
  (return (Variables|Default|GetAttacking)))

(fn IsFlipped
  (return (Variables|Default|GetFlipped)))