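; Spellbook component that automatically casts its spells from the owning actor on a repeating cooldown.
; A looping timer started at BeginPlay calls Cast, which runs its spawn logic only with authority.
; Each cast spawns a SpellStructure at the owner's transform, passes it the Spell data, and starts the spell sequence from the owner's location along its forward vector.
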(event Custom|CastTime
  (CallFunction|Cast))

(event EventBeginPlay
  (Utilities|Time|SetTimerbyEvent (delegate Custom|CastTime) (Variables|Default|GetCooldown) true))

(event EventTick
  (params (DeltaSeconds :type Float%20%28single-precision%29)))

(fn Cast
  (bind _returnvalue (Components|GetOwner))
  (Networking|SwitchHasAuthority
    (:Authority
      (bind _returnvalue_2 (Game|SpawnActorfromClass "/Game/Blueprints/Spells/SpellStructure.SpellStructure_C" (Transformation|GetActorTransform (Components|GetOwner)) "Undefined" "MultiplyWithRoot" 0 (Variables|Default|GetSpell) 0))
      (Default|CastNextSpell _returnvalue_2 -1 (Transformation|GetActorLocation _returnvalue) (Transformation|GetActorForwardVector _returnvalue)))))