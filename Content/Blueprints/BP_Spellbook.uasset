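; Spellbook Blueprint that automatically casts its configured spell on a repeating cooldown.
; A looping timer started on BeginPlay calls Cast, which acts only with network authority.
; Each cast spawns a new SpellStructure at its own transform, passes it the spell data, and calls CastNextSpell from index -1 along its forward vector.
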(event Custom|CastTime
  (CallFunction|Cast))

(event EventBeginPlay
  (Utilities|Time|SetTimerbyEvent (delegate Custom|CastTime) (Variables|Default|GetCooldown) true))

(event Collision|EventActorBeginOverlap
  (params (OtherActor :type Actor%20Object%20Reference)))

(event EventTick
  (params (DeltaSeconds :type Float%20%28single-precision%29)))

(fn ConstructionScript)

(fn Cast
  (Networking|SwitchHasAuthority
    (:Authority
      (bind _returnvalue (Game|SpawnActorfromClass "/Game/Blueprints/Spells/SpellStructure.SpellStructure_C" (Transformation|GetActorTransform) "Undefined" "MultiplyWithRoot" 0 (Variables|Default|GetSpell) 0))
      (Default|CastNextSpell _returnvalue -1 (Transformation|GetActorLocation) (Transformation|GetActorForwardVector)))))