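; Caster component that holds a mana pool, an inventory and spellbooks whose pages each store a spell and its modifiers.
; On authority, Tick regenerates mana, then siphons it into each spellbook in array order, capped by rate, book capacity and remaining pool.
; Events add or remove inventory items, spells and modifiers by index.
; SetSpell and SetModifier edit nested structs through local copies written back to the spellbook.
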(event Custom|ModifierRemove
  (params (Spellbook :type Integer) (Page :type Integer) (Index :type Integer))
  ;[0.15 0.15 0.15 0.5] Inventory setters
  (CallFunction|SetModifier Spellbook Page Index))

(event Custom|InventoryRemove
  (params (Index :type Integer))
  ;[0.15 0.15 0.15 0.5] Inventory setters
  (Utilities|Array|SetArrayElem :TargetArray (Variables|Default|GetInventory) :Index Index))

(event Custom|InventoryAdd
  (params (Index :type Integer) (Item :type Spell%20Item%20Structure))
  ;[0.15 0.15 0.15 0.5] Inventory setters
  (Utilities|Array|SetArrayElem (Variables|Default|GetInventory) Index Item))

(event Custom|SpellRemove
  (params (Spellbook :type Integer) (Page :type Integer))
  ;[0.15 0.15 0.15 0.5] Inventory setters
  (CallFunction|SetSpell Spellbook Page))

(event Custom|ModifierAdd
  (params (Spellbook :type Integer) (Page :type Integer) (Index :type Integer) (Modifier :type Spell%20Item%20Structure))
  ;[0.15 0.15 0.15 0.5] Inventory setters
  (CallFunction|SetModifier Spellbook Page Index Modifier))

(event Custom|SpellAdd
  (params (Spellbook :type Integer) (Page :type Integer) (Spell :type Spell%20Item%20Structure))
  ;[0.15 0.15 0.15 0.5] Inventory setters
  (CallFunction|SetSpell Spellbook Page Spell))

(event EventBeginPlay)

(event EventTick
  (params (DeltaSeconds :type Float%20%28single-precision%29))
  (bind _spellbooks (Variables|Default|GetSpellbooks))
  (Networking|SwitchHasAuthority
    (:Authority
      ;[0.15 0.15 0.15 0.5] regenerate mana
      (Variables|Default|SetMana (+ (Math|Float|Min(Float) (* DeltaSeconds (Variables|Default|GetManaRegenRate)) (- (Variables|Default|GetManaMax) (Variables|Default|GetMana))) (Variables|Default|GetMana)))
      ;[0.15 0.15 0.15 0.5] Siphon mana into spellbooks
      (for (_array_element _array_index) _spellbooks
        (Utilities|Struct|SetmembersinSpellbookData (Utilities|Array|Get(acopy) _spellbooks _array_index) (+ (Math|Float|Min(Float) (* DeltaSeconds (.ManaSiphonRate (Utilities|Struct|BreakSpellbookData _array_element))) (- (.ManaMax (Utilities|Struct|BreakSpellbookData _array_element)) (.Mana (Utilities|Struct|BreakSpellbookData _array_element))) (Variables|Default|GetMana)) (.Mana (Utilities|Struct|BreakSpellbookData _array_element))))
        (Variables|Default|SetMana (- (Variables|Default|GetMana) (Math|Float|Min(Float) (* DeltaSeconds (.ManaSiphonRate (Utilities|Struct|BreakSpellbookData _array_element))) (- (.ManaMax (Utilities|Struct|BreakSpellbookData _array_element)) (.Mana (Utilities|Struct|BreakSpellbookData _array_element))) (Variables|Default|GetMana))))))))

(fn SetModifier
  (params (Spellbook :type Integer) (Page :type Integer) (Index :type Integer) (Modifier :type Spell%20Item%20Structure))
  (bind _spellbooks (Variables|Default|GetSpellbooks))
  (bind _output (Utilities|Array|Get(acopy) _spellbooks Spellbook))
  (bind _output_get (LocalVariables|SetNewLocalVar (.Spells (Utilities|Struct|BreakSpellbookData _output))))
  (bind _output_get_2 (LocalVariables|SetNewLocalVar_0 (.Modifiers (Utilities|Struct|BreakModifiedSpell (Utilities|Array|Get(acopy) _output_get Page)))))
  (Utilities|Array|SetArrayElem _output_get_2 Index Modifier)
  (Utilities|Struct|SetmembersinModifiedSpell (Utilities|Array|Get(acopy) _output_get Page) _output_get_2)
  (Utilities|Struct|SetmembersinSpellbookData _output _output_get))

(fn SetSpell
  (params (Spellbook :type Integer) (Page :type Integer) (Spell :type Spell%20Item%20Structure))
  (bind _spellbooks (Variables|Default|GetSpellbooks))
  (bind _output (Utilities|Array|Get(acopy) _spellbooks Spellbook))
  (bind _output_get (LocalVariables|SetNewLocalVar (.Spells (Utilities|Struct|BreakSpellbookData _output))))
  (Utilities|Struct|SetmembersinModifiedSpell (Utilities|Array|Get(acopy) _output_get Page) Spell)
  (Utilities|Struct|SetmembersinSpellbookData _output _output_get))