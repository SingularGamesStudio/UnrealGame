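; Projectile spell Blueprint that launches a physics shape along its direction at a set speed and applies projectile modifiers every tick.
; A physics behavior setting picks query-only or physical collision, and whether a hit or overlap expires the spell or spawns the next one.
; Hits record location and normal as hints for the next spell's position and direction, which otherwise fall back to the shape's location and parent's direction.
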(event EventBeginPlay
  (|CallParentFunction)
  (CallFunction|SetCollisionBehavior)
  (Physics|SetPhysicsLinearVelocity (Variables|Default|GetPhysicsShape) (* (Variables|Default|GetDirection) (Variables|Default|GetSpeed)) false "None"))

(event EventTick
  (params (DeltaSeconds :type Float%20%28single-precision%29))
  (|CallParentFunction DeltaSeconds)
  (Default|ApplyProjectileModifiers (Variables|Default|GetParent) (Variables|Default|GetIndex) self))

(event Collision|EventHit
  (params (MyComp :type Primitive%20Component%20Object%20Reference) (Other :type Actor%20Object%20Reference) (OtherComp :type Primitive%20Component%20Object%20Reference) (bSelfMoved :type Boolean) (HitLocation :type Vector :default "0, 0, 0") (HitNormal :type Vector :default "0, 0, 0") (NormalImpulse :type Vector :default "0, 0, 0") (Hit :type Hit%20Result%20Structure%20%28by%20ref%29))
  (Variables|Default|SetNextPosHint HitLocation)
  (Variables|Default|SetNextDirHint HitNormal)
  (Utilities|FlowControl|Sequence
    (:then_1
      (switch Utilities|FlowControl|Switch|SwitchonPhysicsBehavior (Variables|Default|GetPhysicsBehavior)
        (:NewEnumerator1
          (CallFunction|Expire))
        (:NewEnumerator3
          (CallFunction|SpawnNextSpell))))))

(event Collision|EventActorBeginOverlap
  (params (OtherActor :type Actor%20Object%20Reference))
  (Utilities|FlowControl|Sequence
    (:then_1
      (switch Utilities|FlowControl|Switch|SwitchonPhysicsBehavior (Variables|Default|GetPhysicsBehavior)
        (:NewEnumerator1
          (CallFunction|Expire))
        (:NewEnumerator3
          (CallFunction|SpawnNextSpell))))))

(fn ConstructionScript
  (|CallParentFunction))

(fn SetCollisionBehavior
  (bind _physicsshape (Variables|Default|GetPhysicsShape))
  (switch Utilities|FlowControl|Switch|SwitchonPhysicsBehavior (Variables|Default|GetPhysicsBehavior)
    (:NewEnumerator0
      (Collision|SetCollisionEnabled _physicsshape "QueryOnly"))
    (:NewEnumerator1
      (Collision|SetCollisionEnabled _physicsshape "QueryAndPhysics" :!label _label))
    (:NewEnumerator2
      (goto _label))
    (:NewEnumerator3
      (goto _label))))

(fn NextPosition
  (bind _nextposhint (Variables|Default|GetNextPosHint))
  (if (Math|Vector|VectorIsNearlyZero _nextposhint)
    (return (Transformation|GetWorldLocation (Variables|Default|GetPhysicsShape)))
    (else
      (return _nextposhint))))

(fn NextDirection
  (bind _nextdirhint (Variables|Default|GetNextDirHint))
  (if (Math|Vector|VectorIsNearlyZero _nextdirhint)
    (bind _direction (|CallParentFunction))
    (return _direction)
    (else
      (return _nextdirhint))))