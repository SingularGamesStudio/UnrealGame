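; Spell-chain actor that runs a sequence of spells with their modifiers and destroys itself once all spawned spells are gone.
; CastNextSpell spawns the next entry's actor, starts its CSpellBase component with itself as parent, and tracks an active count through destroy events.
; Helper functions apply each entry's startup or per-frame projectile modifiers to a given spell.
; Pay deducts mana from the caster's selected spellbook, failing when insufficient.
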(event Custom|ChildDestroyed
  (params (Child :type Actor%20Object%20Reference))
  (bind _output_get (Variables|Default|SetActiveCount (+ (Variables|Default|GetActiveCount) -1)))
  (Math|Integer|CompareInt _output_get
    (:==
      _)
    (:<
      _))
  (Actor|DestroyActor))

(event EventBeginPlay)

(event Collision|EventActorBeginOverlap
  (params (OtherActor :type Actor%20Object%20Reference)))

(event EventTick
  (params (DeltaSeconds :type Float%20%28single-precision%29)))

(fn ConstructionScript)

(fn CastNextSpell
  (params (Index :type Integer) (Position :type Vector) (Direction :type Vector))
  (bind _returnvalue (+ Index 1))
  (bind _spells (Variables|Default|GetSpells))
  (bind _output (Utilities|Array|Get(acopy) _spells _returnvalue))
  (bind _spell (Utilities|Struct|BreakModifiedSpell _output))
  (bind (_sprite _type _spell_2) (Utilities|Struct|BreakSpellItem _spell))
  (Math|Integer|CompareInt _returnvalue (Utilities|Array|Length _spells)
    (:>
      _)
    (:==
      _)
    (:<
      (switch Utilities|FlowControl|Switch|SwitchonSpellItemType _type
        (:NewEnumerator1
          ;[0.15 0.15 0.15 0.5] Instantiate and init fields
          (bind _returnvalue_2 (Game|SpawnActorfromClass _spell_2 (Math|Conversions|ToTransform(Vector) Position) "Undefined" "MultiplyWithRoot" 0 0))
          (Default|Start (Actor|GetComponentbyClass _returnvalue_2 "/Game/Blueprints/Spells/CSpellBase.CSpellBase_C") _returnvalue self Direction)
          ;[0.15 0.15 0.15 0.5] Count active spells
          (Variables|Default|SetActiveCount (+ (Variables|Default|GetActiveCount) 1))
          (Game|BindEventtoOnDestroyed (EventDispatchers|CreateEvent :!event Custom|ChildDestroyed))
          (return true)))))
  (return false))

(fn ApplyStartupModifiers
  (params (Index :type Integer) (Spell :type C%20Spell%20Base%20Object%20Reference))
  (for _array_element (.Modifiers (Utilities|Struct|BreakModifiedSpell (Utilities|Array|Get(acopy) (Variables|Default|GetSpells) Index)))
    (switch Utilities|FlowControl|Switch|SwitchonSpellItemType (.Type (Utilities|Struct|BreakSpellItem _array_element))
      (:NewEnumerator2
        (CallFunction|ApplyStartupModifier (.StartupModifier (Utilities|Struct|BreakSpellItem _array_element)) Spell)))))

(fn ApplyProjectileModifiers
  (params (Index :type Integer) (Spell :type C%20Projectile%20Spell%20Object%20Reference) (DeltaTime :type Float%20%28double-precision%29))
  (for _array_element (.Modifiers (Utilities|Struct|BreakModifiedSpell (Utilities|Array|Get(acopy) (Variables|Default|GetSpells) Index)))
    (switch Utilities|FlowControl|Switch|SwitchonSpellItemType (.Type (Utilities|Struct|BreakSpellItem _array_element))
      (:NewEnumerator3
        (CallFunction|ApplyProjectileModifier (.ProjectileModifier (Utilities|Struct|BreakSpellItem _array_element)) Spell DeltaTime)))))

(fn Pay
  (params (ManaCost :type Float%20%28double-precision%29))
  (bind _caster (Variables|Default|GetCaster))
  (bind _spellbookindex (Variables|Default|GetSpellbookIndex))
  (bind _spellbooks (Variables|/Game/Blueprints/Characters/Player/C_Caster.C_Caster_C|GetSpellbooks _caster))
  (bind _output (Utilities|Array|Get(acopy) _spellbooks _spellbookindex))
  (bind _mana (Utilities|Struct|BreakSpellbookData _output))
  (Math|Float|CompareFloat ManaCost _mana
    (:>
      (return false))
    (:==
      _)
    (:<
      _))
  (Utilities|Struct|SetmembersinSpellbookData _output (- _mana ManaCost))
  (return true))