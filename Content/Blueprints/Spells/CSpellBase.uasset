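; Base spell component that drives one spell in an indexed chain cast by its Parent.
; On authority, Start applies the Parent's startup modifiers, pays mana or destroys the owning actor, sets a lifetime timer unless LifeTime is negative, and optionally calls CallAfterStart.
; Expire asks the Parent to cast the next spell at the owner's location along the stored direction, then calls an empty OnDestroy hook and destroys the owner.
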(event Custom|Expire
  (Networking|SwitchHasAuthority
    (:Authority
      (Utilities|FlowControl|Sequence
        (:then_0
          (CallFunction|SpawnNextSpell))
        (:then_1
          (CallFunction|OnDestroy))
        (:then_2
          (Actor|DestroyActor (Components|GetOwner)))))))

(event EventBeginPlay)

(event EventTick
  (params (DeltaSeconds :type Float%20%28single-precision%29)))

(fn OnDestroy)

(fn SpawnNextSpell
  (bind _direction (CallFunction|NextDirection))
  (bind _direction_2 (CallFunction|NextPosition))
  (Default|CastNextSpell (Variables|Default|GetParent) (Variables|Default|GetIndex) _direction_2 _direction))

(fn NextDirection
  (return (Variables|Default|GetDirection)))

(fn NextPosition
  (return (Transformation|GetActorLocation (Components|GetOwner))))

(fn Start
  (params (Index :type Integer) (Parent :type Spell%20Structure%20Object%20Reference) (Direction :type Vector))
  (bind _lifetime (Variables|Default|GetLifeTime))
  (Variables|Default|SetIndex Index)
  (Variables|Default|SetParent Parent)
  (Variables|Default|SetDirection Direction)
  (Networking|SwitchHasAuthority
    (:Authority
      (Utilities|FlowControl|Sequence
        (:then_0
          (Default|ApplyStartupModifiers (Variables|Default|GetParent) (Variables|Default|GetIndex) self))
        (:then_1
          ;[0.15 0.15 0.15 0.5] Pay mana
          (bind _successful (Default|Pay (Variables|Default|GetParent) (Variables|Default|GetManacost)))
          (if (not _successful)
            (Actor|DestroyActor (Components|GetOwner))))
        (:then_2
          ;[0.15 0.15 0.15 0.5] expiration trigger
          (Math|Float|CompareFloat _lifetime 0.0
            (:>
              _)
            (:==
              _))
          (bind _returnvalue (Utilities|Time|SetTimerbyEvent (EventDispatchers|CreateEvent :!event Custom|Expire) _lifetime))
          (Variables|Default|SetTimer _returnvalue))
        (:then_3
          (if (Variables|Default|GetEmitStart)
            (Default|CallAfterStart)))))))