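; Spell modifier function library that alters spell speed and projectile physics behavior based on a modifier value.
; ApplyStartupModifier calls SFast to boost speed, while ApplyProjectileModifier dispatches to Antigravity or Chaotic handlers, with S and P as empty stubs.
; The sign of DeltaTime gates projectile effects: negative disables gravity for Antigravity, positive lets Chaotic randomly deflect velocity.
; Chaotic applies the difference between rotated and current velocity as a velocity-change impulse.
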(fn ApplyStartupModifier
  (params (Modifier :type StartupModifier%20Enum :default "NewEnumerator0") (Spell :type C%20Spell%20Base%20Object%20Reference%20%28by%20ref%29))
  (switch Utilities|FlowControl|Switch|SwitchonStartupModifier Modifier
    (:NewEnumerator0
      (CallFunction|SFast Spell))))

(fn ApplyProjectileModifier
  (params (Modifier :type ProjectileModifier%20Enum :default "ProjectileModifier_MAX") (Spell :type C%20Projectile%20Spell%20Object%20Reference%20%28by%20ref%29) (DeltaTime :type Float%20%28double-precision%29))
  (switch Utilities|FlowControl|Switch|SwitchonProjectileModifier Modifier
    (:NewEnumerator2
      (CallFunction|PAntigravity Spell DeltaTime))
    (:NewEnumerator4
      (CallFunction|PChaotic Spell DeltaTime))))

(fn SFast
  (params (Spell :type C%20Spell%20Base%20Object%20Reference%20%28by%20ref%29))
  (Math|Float|CompareFloat (Math|Float|Absolute(Float) (Variables|/Game/Blueprints/Spells/CSpellBase.CSpellBase_C|GetSpeed Spell)) 1.0
    (:>
      (Variables|/Game/Blueprints/Spells/CSpellBase.CSpellBase_C|SetSpeed Spell (* (Variables|/Game/Blueprints/Spells/CSpellBase.CSpellBase_C|GetSpeed Spell) 2.0) :!label _label))
    (:==
      (goto _label))
    (:<
      (Variables|/Game/Blueprints/Spells/CSpellBase.CSpellBase_C|SetSpeed Spell (+ (Variables|/Game/Blueprints/Spells/CSpellBase.CSpellBase_C|GetSpeed Spell) (Math|Float|Sign(Float) (Variables|/Game/Blueprints/Spells/CSpellBase.CSpellBase_C|GetSpeed Spell)) (== (Variables|/Game/Blueprints/Spells/CSpellBase.CSpellBase_C|GetSpeed Spell) 0.0))))))

(fn S
  (params (Spell :type C%20Spell%20Base%20Object%20Reference%20%28by%20ref%29)))

(fn P
  (params (Spell :type C%20Projectile%20Spell%20Object%20Reference%20%28by%20ref%29) (DeltaTime :type Float%20%28double-precision%29)))

(fn PAntigravity
  (params (Spell :type C%20Projectile%20Spell%20Object%20Reference%20%28by%20ref%29) (DeltaTime :type Float%20%28double-precision%29))
  (Math|Float|CompareFloat DeltaTime 0.0
    (:<
      (Physics|SetEnableGravity (Variables|/Game/Blueprints/Spells/CProjectileSpell.CProjectileSpell_C|GetPhysicsShape Spell) false))))

(fn PChaotic
  (params (Spell :type C%20Projectile%20Spell%20Object%20Reference%20%28by%20ref%29) (DeltaTime :type Float%20%28double-precision%29))
  (bind _physicsshape (Variables|/Game/Blueprints/Spells/CProjectileSpell.CProjectileSpell_C|GetPhysicsShape Spell))
  (Math|Float|CompareFloat DeltaTime 0.0
    (:>
      (bind _returnvalue (Physics|GetPhysicsLinearVelocity _physicsshape "None"))
      (Physics|AddImpulse _physicsshape (- (Math|Vector|RotateVectorAroundAxis _returnvalue (Math|Random|RandomFloatinRange -2e+01 2e+01) (Math|Vector|Normalize (Math|Vector|CrossProduct (Math|Vector|Normalize _returnvalue) (Math|Random|RandomUnitVector)))) _returnvalue) "None" true))))