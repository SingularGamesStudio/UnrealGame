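; Projectile spell component that launches its owner's physics primitive along a direction at a set speed as part of a spell chain.
; PhysicsBehavior sets collision and whether a hit expires the spell, spawns the next one or does neither.
; On authority, hits apply WeakDamage and record location and normal as hints for the next spell's position and direction.
; The parent applies projectile modifiers at start and every tick, also only on authority.
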(event Custom|CustomEvent
  (params (SelfActor :type Actor%20Object%20Reference) (OtherActor :type Actor%20Object%20Reference) (NormalImpulse :type Vector) (Hit :type Hit%20Result%20Structure%20%28by%20ref%29))
  (bind (_bblockinghit _binitialoverlap _time _distance _location _impactpoint _normal) (Collision|BreakHitResult Hit))
  (Networking|SwitchHasAuthority
    (:Authority
      (Variables|Default|SetNext%20Pos%20Hint _location)
      (Variables|Default|SetNext%20Dir%20Hint _normal)
      (Utilities|FlowControl|Sequence
        (:then_0
          (Game|Damage|ApplyDamage OtherActor (Variables|Default|GetDamage) (Variables|/Game/Blueprints/Spells/SpellStructure.SpellStructure_C|GetDamageOwner (Variables|Default|GetParent)) (Components|GetOwner) "/Game/Blueprints/WeakDamage.WeakDamage_C"))
        (:then_1
          (switch Utilities|FlowControl|Switch|SwitchonPhysicsBehavior (Variables|Default|GetPhysicsBehavior)
            (:NewEnumerator1
              (CallFunction|Expire))
            (:NewEnumerator3
              (CallFunction|SpawnNextSpell))))))))

(event EventBeginPlay
  (Collision|BindEventtoOnActorHit (Components|GetOwner) (delegate Custom|CustomEvent)))

(event EventTick
  (params (DeltaSeconds :type Float%20%28single-precision%29))
  (|CallParentFunction DeltaSeconds)
  (Networking|SwitchHasAuthority
    (:Authority
      (Default|ApplyProjectileModifiers (Variables|Default|GetParent) (Variables|Default|GetIndex) self DeltaSeconds))))

(fn SetCollisionBehavior
  (bind _physicsshape (Variables|Default|GetPhysicsShape))
  (switch Utilities|FlowControl|Switch|SwitchonPhysicsBehavior (Variables|Default|GetPhysicsBehavior)
    (:NewEnumerator0
      (Collision|SetCollisionEnabled _physicsshape "QueryOnly"))
    (:NewEnumerator1
      (Collision|SetCollisionEnabled _physicsshape "QueryAndPhysics" :!label _label))
    (:NewEnumerator2
      (goto _label))
    (:NewEnumerator3
      (goto _label))))

(fn NextPosition
  (bind _next_pos_hint (Variables|Default|GetNext%20Pos%20Hint))
  (if (Math|Vector|VectorIsNearlyZero _next_pos_hint)
    (return (Transformation|GetWorldLocation (Variables|Default|GetPhysicsShape)))
    (else
      (return _next_pos_hint))))

(fn NextDirection
  (bind _next_dir_hint (Variables|Default|GetNext%20Dir%20Hint))
  (if (Math|Vector|VectorIsNearlyZero _next_dir_hint)
    (bind _direction (|CallParentFunction))
    (return _direction)
    (else
      (return _next_dir_hint))))

(fn Start
  (params (Index :type Integer) (Parent :type Spell%20Structure%20Object%20Reference) (Direction :type Vector :default "0, 0, 0"))
  (|CallParentFunction Index Parent Direction)
  (Utilities|FlowControl|Sequence
    (:then_0
      (bind _output_get (Variables|Default|SetPhysicsShape (Actor|GetComponentbyClass (Components|GetOwner) "/Script/Engine.PrimitiveComponent")))
      (CallFunction|SetCollisionBehavior)
      (Physics|SetPhysicsLinearVelocity _output_get (* (Variables|Default|GetDirection) (Variables|Default|GetSpeed)) false "None")
      (Default|CallAfterStart))
    (:then_1
      (Networking|SwitchHasAuthority
        (:Authority
          (Default|ApplyProjectileModifiers (Variables|Default|GetParent) (Variables|Default|GetIndex) self -1.0))))))