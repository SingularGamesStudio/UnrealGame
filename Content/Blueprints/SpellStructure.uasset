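; SpellStructure is an actor that holds a sequence of spells and manages the lifetime of the spell actors it spawns.
; CastNextSpell spawns the spell following a given index at a position, passing it direction, index and parent, and returns false when no valid spell remains.
; A counter tracks live spawned spells through their destroyed events, and the structure destroys itself when ChildDestroyed brings it to zero or below.
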(event Custom|ChildDestroyed
  (params (Child :type Actor%20Object%20Reference))
  (bind _output_get (Variables|Default|SetActiveCount (+ (Variables|Default|GetActiveCount) -1)))
  (Math|Integer|CompareInt _output_get
    (:==
      _)
    (:<
      _))
  (Actor|DestroyActor))

(event EventBeginPlay)

(event Collision|EventActorBeginOverlap
  (params (OtherActor :type Actor%20Object%20Reference)))

(event EventTick
  (params (DeltaSeconds :type Float%20%28single-precision%29)))

(fn ConstructionScript)

(fn CastNextSpell
  (params (Index :type Integer) (Position :type Vector) (Direction :type Vector))
  (bind _returnvalue (+ Index 1))
  (bind _spells (Variables|Default|GetSpells))
  (bind _output (Utilities|Array|Get(acopy) _spells _returnvalue))
  (bind _spell (Utilities|Struct|BreakModifiedSpell _output))
  (Math|Integer|CompareInt _returnvalue (Utilities|Array|Length _spells)
    (:>
      _)
    (:==
      _)
    (:<
      (if (Utilities|IsValidClass _spell)
        (bind _returnvalue_2 (Game|SpawnActorfromClass _spell (Math|Conversions|ToTransform(Vector) Position) "Undefined" "MultiplyWithRoot" 0 Direction _returnvalue self 0))
        (Variables|Default|SetActiveCount (+ (Variables|Default|GetActiveCount) 1))
        (Game|BindEventtoOnDestroyed _returnvalue_2 (EventDispatchers|CreateEvent :!event Custom|ChildDestroyed))
        (return true)
        (else
          _))))
  (return false))