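; Base actor for spells in a chained casting sequence, with empty OnStart, OnTick and OnDestroy hooks for child spells to override.
; BeginPlay sets an expiration timer unless LifeTime is negative, then calls OnStart.
; Expire asks Parent to cast the next spell using this one's Index, location and NextDirection, then runs OnDestroy and destroys the actor.
; NextDirection returns Direction by default.
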(event Custom|Expire
  (Utilities|FlowControl|Sequence
    (:then_0
      (CallFunction|SpawnNextSpell))
    (:then_1
      (CallFunction|OnDestroy))
    (:then_2
      (Actor|DestroyActor))))

(event EventBeginPlay
  (bind _lifetime (Variables|Default|GetLifeTime))
  (Utilities|FlowControl|Sequence
    (:then_0
      ;[0.15 0.15 0.15 0.5] expiration trigger
      (Math|Float|CompareFloat _lifetime 0.0
        (:>
          _)
        (:==
          _))
      (bind _returnvalue (Utilities|Time|SetTimerbyEvent (EventDispatchers|CreateEvent :!event Custom|Expire) _lifetime))
      (Variables|Default|SetTimer _returnvalue))
    (:then_1
      (CallFunction|OnStart))))

(event Collision|EventActorBeginOverlap
  (params (OtherActor :type Actor%20Object%20Reference)))

(event EventTick
  (params (DeltaSeconds :type Float%20%28single-precision%29))
  (CallFunction|OnTick DeltaSeconds))

(fn ConstructionScript)

(fn OnStart)

(fn OnDestroy)

(fn OnTick
  (params (deltaTime :type Float%20%28double-precision%29)))

(fn NextDirection
  (return (Variables|Default|GetDirection)))

(fn SpawnNextSpell
  (bind _direction (CallFunction|NextDirection))
  (Default|CastNextSpell (Variables|Default|GetParent) (Variables|Default|GetIndex) (Transformation|GetActorLocation) _direction))