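; Base character with team-filtered damage, knockback, health and ragdoll death.
; Possession copies the team ID from the AI or player controller; enemy damage reduces health and launches the character, mirroring its velocity off hit surfaces during a short bounce window.
; At zero health it ragdolls with the hit impulse and unregisters from AI perception.
; While alive, optional Tick logic yaws the mesh from target and movement directions for the animation blendspace.
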(event Custom|Take%20Damage
  (params (DamagedActor :type Actor%20Object%20Reference) (Damage :type Float%20%28single-precision%29) (DamageType :type Damage%20Type%20Object%20Reference) (InstigatedBy :type Controller%20Object%20Reference) (DamageCauser :type Actor%20Object%20Reference))
  (bind _returnvalue (Transformation|GetActorLocation DamageCauser))
  (bind _returnvalue_2 (Transformation|GetActorLocation))
  (bind _damageimpulse (Variables|/Script/Engine.DamageType|GetDamageImpulse DamageType))
  (bind _returnvalue_3 (- _returnvalue_2 _returnvalue))
  (bind _returnvalue_4 (Math|Vector|Normalize _returnvalue_3))
  (bind _returnvalue_5 (* _returnvalue_4 _damageimpulse Damage))
  ;[0.15 0.15 0.15 0.5] Check teams
  (bind _asmy_aicontroller (Utilities|Casting|CastToMyAIController InstigatedBy)
    (:then
      (if (!= (Variables|/Script/UnrealGame.MyAIController|GetTeamId _asmy_aicontroller) (Variables|Default|GetTeamID))
        (Utilities|FlowControl|Sequence :!label _label
          (:then_0
            ;[0.15 0.15 0.15 0.5] Take damage
            (Variables|Default|SetHealth (- (Variables|Default|GetHealth) Damage)))
          (:then_1
            ;[0.15 0.15 0.15 0.5] Bounce
            (Variables|Default|SetDamageBounce true)
            (Variables|Default|SetHitVelocity _returnvalue_5)
            (Character|LaunchCharacter _returnvalue_5 false false)
            (bind _returnvalue_6 (Utilities|Time|SetTimerbyEvent (delegate Custom|ResetBounce) 0.5))
            (Variables|Default|SetBounceTimer _returnvalue_6))
          (:then_2
            ;[0.15 0.15 0.15 0.5] Death
            (Math|Float|CompareFloat (Variables|Default|GetHealth) 0.0
              (:==
                _)
              (:<
                _))
            (CallFunction|OnDeath)))))
    (:CastFailed
      (bind _asmy_player_controller (Utilities|Casting|CastToMyPlayerController InstigatedBy))
      (if (!= (Variables|/Script/UnrealGame.MyPlayerController|GetTeamId _asmy_player_controller) (Variables|Default|GetTeamID))
        (goto _label)))))

(event Custom|Ragdoll
  (CallFunction|RagdollStart))

(event Custom|ResetBounce
  ;[0.15 0.15 0.15 0.5] Bounce
  (Variables|Default|SetDamageBounce false))

(event EventBeginPlay
  (Variables|Default|SetInitialRotation (.Yaw (Math|Rotator|BreakRotator (Variables|/Script/Engine.SceneComponent|GetRelativeRotation (Variables|Character|GetMesh)))))
  (EventDispatchers|BindEventtoOnTakeAnyDamage (delegate Custom|Take%20Damage))
  (Variables|Default|SetHealth (Variables|Default|GetMaxHealth)))

(event Collision|EventActorBeginOverlap
  (params (OtherActor :type Actor%20Object%20Reference)))

(event EventTick
  (params (DeltaSeconds :type Float%20%28single-precision%29))
  (bind _returnvalue (Transformation|GetActorLocation))
  (bind _charactermovement (Variables|Character|GetCharacterMovement))
  (bind _velocity (Variables|/Script/Engine.MovementComponent|GetVelocity _charactermovement))
  (bind (_x _y) (Math|Vector|BreakVector _velocity))
  (bind _returnvalue_2 (Math|Vector|MakeVector _x _y 0.0))
  (bind _returnvalue_3 (Math|Vector|Normalize _returnvalue_2))
  (if (not (Variables|Default|GetDead))
    ;[0.15 0.15 0.15 0.5] Mesh must be oriented towards look direction for animation blendspace to work correctly (already true for player)
    (if (Variables|Default|GetControlRotation)
      (bind _forward (CallFunction|GetLookDirection))
      (Transformation|SetRelativeRotation (Variables|Character|GetMesh) (Math|Rotator|MakeRotator 0.0 0.0 (+ (* (Math|Float|Clamp(Float) (Class|KismetMathLibrary|DegAtan2 (Class|KismetMathLibrary|CrossProduct2D (Math|Conversions|ToVector2D(Vector) (Math|Vector|Normalize (Math|Vector|MakeVector (.X (Math|Vector|BreakVector _forward)) (.Y (Math|Vector|BreakVector _forward)) 0.0))) (Math|Conversions|ToVector2D(Vector) _returnvalue_3)) (Math|Vector|DotProduct (Math|Vector|Normalize (Math|Vector|MakeVector (.X (Math|Vector|BreakVector _forward)) (.Y (Math|Vector|BreakVector _forward)) 0.0)) _returnvalue_3)) -9e+01 9e+01) -1.0) (Variables|Default|GetInitialRotation))) false false)
      (Networking|SwitchHasAuthority
        (:Authority
          (Rendering|Debug|DrawDebugArrow :LineStart _returnvalue :LineEnd (+ _forward _returnvalue) :ArrowSize 1e+02))))))

(event EventPossessed
  (params (NewController :type Controller%20Object%20Reference))
  ;[0.15 0.15 0.15 0.5] Save team id
  (bind _asmy_aicontroller (Utilities|Casting|CastToMyAIController NewController)
    (:then
      (Variables|Default|SetTeamID (Variables|/Script/UnrealGame.MyAIController|GetTeamId _asmy_aicontroller)))
    (:CastFailed
      (bind _asmy_player_controller (Utilities|Casting|CastToMyPlayerController NewController))
      (Variables|Default|SetTeamID (Variables|/Script/UnrealGame.MyPlayerController|GetTeamId _asmy_player_controller)))))

(event Collision|EventHit
  (params (MyComp :type Primitive%20Component%20Object%20Reference) (Other :type Actor%20Object%20Reference) (OtherComp :type Primitive%20Component%20Object%20Reference) (bSelfMoved :type Boolean) (HitLocation :type Vector :default "0, 0, 0") (HitNormal :type Vector :default "0, 0, 0") (NormalImpulse :type Vector :default "0, 0, 0") (Hit :type Hit%20Result%20Structure%20%28by%20ref%29))
  (if (Variables|Default|GetDamageBounce)
    (Character|LaunchCharacter (Math|Vector|MirrorVectorbyNormal (Variables|Default|GetHitVelocity) HitNormal) true true)))

(fn ConstructionScript)

(fn OnDeath
  (Variables|Default|SetDead true)
  (Default|CallDeath)
  (CallFunction|Ragdoll))

(fn RagdollStart
  (bind _mesh (Variables|Character|GetMesh))
  (bind _capsulecomponent (Variables|Collision|GetCapsuleComponent))
  (bind _mesh_2 (Variables|Character|GetMesh))
  (Collision|SetCollisionEnabled _capsulecomponent "NoCollision")
  (Physics|SetSimulatePhysics _capsulecomponent false)
  (Collision|SetCollisionEnabled _mesh "QueryAndPhysics")
  (Collision|SetCollisionProfileName _mesh "Ragdoll" true :!class /Script/Engine.PrimitiveComponent)
  (Physics|SetSimulatePhysics _mesh true)
  (Class|SkeletalMeshComponent|SetEnableAnimation _mesh_2 false)
  (Class|PrimitiveComponent|WakeAllRigidBodies _mesh_2)
  (Physics|AddImpulse (Variables|Character|GetMesh) (* (Variables|Default|GetHitVelocity) 1e+01) "None" true)
  (Variables|Default|SetDamageBounce true)
  (Class|AIPerceptionStimuliSourceComponent|UnregisterfromPerceptionSystem (Variables|Default|GetAIPerceptionStimuliSource)))

(fn GetLookDirection
  (bind _target (Variables|Default|GetTarget))
  (Utilities|IsValid _target
    (:Is%20Valid
      (return (- (Transformation|GetActorLocation _target) (Transformation|GetActorLocation))))
    (:Is%20Not%20Valid
      (return (Transformation|GetActorForwardVector)))))

(fn IsAttacking
  (return (Variables|Default|GetAttacking)))

(fn IsFlipped
  (return (Variables|Default|GetFlipped)))